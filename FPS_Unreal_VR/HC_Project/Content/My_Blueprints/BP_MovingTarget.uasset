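; Shooting target actor that patrols back and forth and counts toward the player's goal when destroyed by projectiles.
; Tick offsets it along Direction at Speed without delta-time scaling, and a looping timer reverses Direction.
; Near-duplicate actor and component hit handlers reduce TargetHealth on projectile hits.
; A hit at zero health or below increments the character's TargetsHit, calls CheckGoal and destroys the target.
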(event OnComponentHit(StaticMesh)
  (params (HitComponent :type Primitive%20Component%20Object%20Reference) (OtherActor :type Actor%20Object%20Reference) (OtherComp :type Primitive%20Component%20Object%20Reference) (NormalImpulse :type Vector :default "0, 0, 0") (Hit :type Hit%20Result%20Structure%20%28by%20ref%29))
  (Utilities|Casting|CastToBP_FirstPersonProjectile OtherActor)
  (Game|Damage|ApplyDamage self 25.0 0 0)
  (bind _asbp_first_person_character (Utilities|Casting|CastToBP_FirstPersonCharacter (Game|GetPlayerCharacter 0)))
  (if (> (Variables|Default|GetTarget%20Health) 0)
    (Variables|Default|SetTarget%20Health (- (Variables|Default|GetTarget%20Health) 25))
    (else
      (Variables|/Game/FirstPerson/Blueprints/BP_FirstPersonCharacter.BP_FirstPersonCharacter_C|SetTargetsHit _asbp_first_person_character (+ (Variables|/Game/FirstPerson/Blueprints/BP_FirstPersonCharacter.BP_FirstPersonCharacter_C|GetTargetsHit _asbp_first_person_character) 1))
      (Default|CheckGoal _asbp_first_person_character)
      (Actor|DestroyActor))))

(event Custom|reversedirection
  ;[0.1823 0.1823 0.1823] Movement
  (Variables|Default|SetDirection (* (Variables|Default|GetDirection) -1.0)))

(event Collision|EventHit
  (params (MyComp :type Primitive%20Component%20Object%20Reference) (Other :type Actor%20Object%20Reference) (OtherComp :type Primitive%20Component%20Object%20Reference) (bSelfMoved :type Boolean) (HitLocation :type Vector :default "0, 0, 0") (HitNormal :type Vector :default "0, 0, 0") (NormalImpulse :type Vector :default "0, 0, 0") (Hit :type Hit%20Result%20Structure%20%28by%20ref%29))
  (Utilities|Casting|CastToBP_FirstPersonProjectile Other)
  (bind _asbp_first_person_character (Utilities|Casting|CastToBP_FirstPersonCharacter (Game|GetPlayerCharacter 0)))
  (if (> (Variables|Default|GetTarget%20Health) 0)
    (Variables|Default|SetTarget%20Health (- (Variables|Default|GetTarget%20Health) 25))
    (else
      (Variables|/Game/FirstPerson/Blueprints/BP_FirstPersonCharacter.BP_FirstPersonCharacter_C|SetTargetsHit _asbp_first_person_character (+ (Variables|/Game/FirstPerson/Blueprints/BP_FirstPersonCharacter.BP_FirstPersonCharacter_C|GetTargetsHit _asbp_first_person_character) 1))
      (Default|CheckGoal _asbp_first_person_character)
      (Actor|DestroyActor))))

(event EventTick
  (params (DeltaSeconds :type Float%20%28single-precision%29))
  ;[0.1823 0.1823 0.1823] Movement
  (Transformation|AddActorWorldOffset (* (Math|Vector|Normalize (Variables|Default|GetDirection)) (Variables|Default|GetSpeed))))

(event EventBeginPlay
  ;[0.1823 0.1823 0.1823] Movement
  (Utilities|Time|SetTimerbyEvent (delegate Custom|reversedirection) (Variables|Default|GetTime%20to%20Change) true))

(fn ConstructionScript)